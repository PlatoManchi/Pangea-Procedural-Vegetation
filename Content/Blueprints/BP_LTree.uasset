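; BP_LTree is an L-system tree actor, by its naming, displayed through a procedural mesh component.
; The construction script calls UpdateLString, defined outside this file, then SetMaterialForLines.
; SetMaterialForLines loops over the mesh sections, alternating red and blue material instances by even and odd index.
; It has no runtime logic, as the event graph holds only disabled placeholder events.
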(fn `SetMaterialForLines`
  (for _index (range (`self.SectionsCount`))
    (if (== (mod _index 2) 0)
      (`PrimitiveComponent.SetMaterial` (`self.proceduralMeshComponent`) _index "/Game/Art/RedMaterial_Inst.RedMaterial_Inst")
      (else
        (`PrimitiveComponent.SetMaterial` (`self.proceduralMeshComponent`) _index "/Game/Art/BlueMaterial_Inst_Inst.BlueMaterial_Inst_Inst")))))

(fn `UserConstructionScript`
  (`self.UpdateLString`)
  (`self.SetMaterialForLines`))